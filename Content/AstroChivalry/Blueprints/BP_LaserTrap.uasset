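; Spinning laser trap that damages whatever its two beams hit.
; Each Tick rotates the mesh by a fixed, frame-rate-dependent step, then line traces forward from two laser location components, applying damage to the hit actor every frame with debug drawing on.
; Both beam effects activate on BeginPlay and have their BeamEnd set to the full trace distance each frame, so they are not shortened at impacts.
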(event `self.ReceiveBeginPlay`
  (`parent.ReceiveBeginPlay`)
  (`ActorComponent.Activate` (`self.Laser1`) false)
  (`ActorComponent.Activate` (`self.Laser2`) false))

(event `self.ReceiveTick`
  (params (DeltaSeconds :type "Float (single-precision)"))
  (bind _laserloc1 (`self.LaserLoc1`))
  (bind _laserloc2 (`self.LaserLoc2`))
  (bind _returnvalue (`SceneComponent.K2_GetComponentLocation` _laserloc2))
  (bind _returnvalue_2 (`SceneComponent.K2_GetComponentLocation` _laserloc1))
  (bind _returnvalue_3 (+ _returnvalue (* (`SceneComponent.GetForwardVector` _laserloc2) 1000.0)))
  (bind _returnvalue_4 (+ _returnvalue_2 (* (`SceneComponent.GetForwardVector` _laserloc1) 1000.0)))
  (`parent.ReceiveTick` DeltaSeconds)
  (`|ExecutionSequence`
    (:`then_0`
      (`SceneComponent.K2_AddLocalRotation` (`self.Mesh`) (struct :`Yaw` 5.0) false false))
    (:`then_1`
      (bind _outhit (`KismetSystemLibrary.LineTraceSingleByProfile` :`Start` _returnvalue_2 :`End` _returnvalue_4 :`ProfileName` "WorldDynamic" :`DrawDebugType` "ForOneFrame"))
      (`GameplayStatics.ApplyDamage` (`.HitActor` (`GameplayStatics.BreakHitResult` _outhit)) 1.0 null self)
      (`NiagaraComponent.SetVariableVec3` (`self.Laser1`) "BeamEnd" _returnvalue_4))
    (:`then_2`
      (bind _outhit_2 (`KismetSystemLibrary.LineTraceSingleByProfile` :`Start` _returnvalue :`End` _returnvalue_3 :`ProfileName` "WorldDynamic" :`DrawDebugType` "ForOneFrame"))
      (`GameplayStatics.ApplyDamage` (`.HitActor` (`GameplayStatics.BreakHitResult` _outhit_2)) 1.0 null self)
      (`NiagaraComponent.SetVariableVec3` (`self.Laser2`) "BeamEnd" _returnvalue_3))))

(fn `UserConstructionScript`
  (`parent.UserConstructionScript`))
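; Cannon projectile that flies to a target location and explodes with full radial damage, attributed to player 0's pawn.
; StartTracking drives a Timeline that lerps the actor from its start point without sweeping.
; Timeline finish or a Sphere hit applies damage, prints debug info, draws the radius, hides Sphere1, disables collision and activates particles, destroying the actor when they finish.
; A hit does not stop the Timeline.
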(event `StartTracking`
  (params (TargetLocation :type "Vector Structure"))
  (bind _returnvalue (`self.K2_GetActorLocation`))
  (bind _particlesystem (`self.ParticleSystem`))
  (bind _output_get (set `self.InitialLocation` (`self.K2_GetActorLocation`)))
  (bind (_direction _alpha) (`Timeline|Timeline`)
    (:`Update`
      (`self.K2_SetActorLocation` (`KismetMathLibrary.VLerp` _output_get TargetLocation _alpha)))
    (:`Finished`
      (bind _returnvalue_2 (`GameplayStatics.ApplyRadialDamage` 150.0 _returnvalue 500.0 null (`|MakeArray` self) (`GameplayStatics.GetPlayerPawn` 0) null true))
      (`KismetSystemLibrary.PrintString` (`KismetStringLibrary.Conv_BoolToString` _returnvalue_2))
      (`KismetSystemLibrary.DrawDebugSphere` _returnvalue 500.0 12 (struct :`R` 1.0 :`G` 1.0 :`B` 1.0 :`A` 1.0) 5.0)
      (`ActorComponent.Activate` _particlesystem true :!label _label)
      (`SceneComponent.SetVisibility` (`self.Sphere1`) false false)
      (`PrimitiveComponent.SetCollisionEnabled` (`self.Sphere`) "NoCollision")
      (add `ParticleSystemComponent.OnSystemFinished` _particlesystem (delegate `CustomEvent`)))))

(event `self.Sphere.OnComponentHit`
  (params (HitComponent :type "PrimitiveComponent Object Reference") (OtherActor :type "Actor Object Reference") (OtherComp :type "PrimitiveComponent Object Reference") (NormalImpulse :type "Vector Structure") (Hit :type "HitResult Structure (by ref)"))
  (`KismetSystemLibrary.PrintString` (`KismetSystemLibrary.GetDisplayName` OtherActor))
  (bind _returnvalue (`GameplayStatics.ApplyRadialDamage` 150.0 Hit_Location 500.0 null (`|MakeArray` self :!type "Actor Object Reference") (`GameplayStatics.GetPlayerPawn` 0) null true))
  (`KismetSystemLibrary.PrintString` (`KismetStringLibrary.Conv_BoolToString` _returnvalue))
  (`KismetSystemLibrary.DrawDebugSphere` Hit_Location 500.0 12 (struct :`R` 1.0 :`G` 1.0 :`B` 1.0 :`A` 1.0) 5.0)
  (goto _label))

(event `CustomEvent`
  (params (PSystem :type "ParticleSystemComponent Object Reference"))
  (`self.K2_DestroyActor`))

(fn `UserConstructionScript`)
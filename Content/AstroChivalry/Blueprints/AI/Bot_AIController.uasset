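; AI controller for bots that runs the BT_BaseBot behavior tree and picks their target.
; AI perception of the player or a structure sets the TargetActor blackboard key and focus, and losing sight starts a three-second timer that clears both.
; Callable functions let structures or objectives be set as the target directly.
; Once an objective is found, the lose-target logic no longer clears it.
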(event `self.ReceiveBeginPlay`
  (`self.RunBehaviorTree` "/Game/AstroChivalry/Blueprints/AI/BT_BaseBot.BT_BaseBot"))

(event `self.AIPerception.OnTargetPerceptionUpdated`
  (params (Actor :type "Actor Object Reference") (Stimulus :type "AIStimulus Structure"))
  (bind (_age _expirationage _strength _stimuluslocation _receiverlocation _tag _bsuccessfullysensed) (break `AIStimulus` Stimulus))
  (bind _output_get (set `self.SensedActor` Actor))
  (cast `/Game/AstroChivalry/Blueprints/Structure` _output_get
    (:`then`
      (bind _output_get_2 (set `self.Found Structure` true)))
    (:`CastFailed`
      _))
  (bind _returnvalue (== _output_get (`GameplayStatics.GetPlayerCharacter` 0)))
  (set `self.Found Player` _returnvalue)
  (if (or _output_get_2 _returnvalue)
    (if _bsuccessfullysensed
      (set `self.Found Structure` (== _tag "Structure"))
      (if (and (`self.Found Player`) (not (`self.Found Objective`)))
        (set `self.SensedActor` (`GameplayStatics.GetPlayerCharacter` 0)))
      (`BlackboardComponent.SetValueAsObject` (`self.Blackboard`) "TargetActor" (`self.SensedActor`))
      (`self.K2_SetFocus` (`self.SensedActor`))
      (`KismetSystemLibrary.K2_ClearAndInvalidateTimerHandle` (`self.LoseTargetTimer`))
      (else
        (bind _returnvalue_2 (`KismetSystemLibrary.K2_SetTimerDelegate` (delegate `LoseTarget`) 3.0))
        (set `self.LoseTargetTimer` _returnvalue_2)))))

(event `LoseTarget`
  (if (not (`self.Found Objective`))
    (`BlackboardComponent.SetValueAsObject` (`self.Blackboard`) "TargetActor" null)
    (`self.K2_ClearFocus`)
    (set `self.Found Player` false)
    (set `self.Found Structure` false)))

(fn `FoundObjective`
  (params (Structure :type "Actor Object Reference"))
  (set `self.SensedActor` Structure)
  (set `self.Found Objective` true)
  (`BlackboardComponent.SetValueAsObject` (`self.Blackboard`) "TargetActor" (`self.SensedActor`))
  (`self.K2_SetFocus` (`self.SensedActor`))
  (`KismetSystemLibrary.K2_ClearAndInvalidateTimerHandle` (`self.LoseTargetTimer`)))

(fn `FoundStructure`
  (params (Structure :type "Actor Object Reference"))
  (set `self.SensedActor` Structure)
  (set `self.Found Structure` true)
  (`BlackboardComponent.SetValueAsObject` (`self.Blackboard`) "TargetActor" (`self.SensedActor`))
  (`self.K2_SetFocus` (`self.SensedActor`))
  (`KismetSystemLibrary.K2_ClearAndInvalidateTimerHandle` (`self.LoseTargetTimer`)))

(fn `LostStructure`
  (`self.LoseTarget`))

(fn `UserConstructionScript`)
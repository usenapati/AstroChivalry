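; Enemy manager that spawns KoboldBot or KnightBot AI, chosen by IsKnight, starting after an initial delay.
; BeginPlay picks a random initial set of active BP_EnemySpawners, then seeds the stream used for random points in their volumes.
; Each spawn sets a non-looping timer, decrements the cooldown, may activate another spawner behind a never-reset HasAdded flag, then calls SpawnEnemy again directly.
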(event `self.ReceiveBeginPlay`
  (`self.Initialize`)
  (`KismetSystemLibrary.Delay` (`self.InitialSpawnDelay`))
  (`self.Spawn Enemy`))

(event `Spawn Enemy`
  (if (`self.IsKnight`)
    (`AIBlueprintHelperLibrary.SpawnAIFromClass` (`self.KoboldBot`) "/Game/AstroChivalry/Blueprints/AI/BT_BaseBot.BT_BaseBot" (`self.GetRandomSpawnPoint`) (struct) false null)
    (else
      (`AIBlueprintHelperLibrary.SpawnAIFromClass` (`self.KnightBot`) null (`self.GetRandomSpawnPoint`) (struct) false null)))
  (`KismetSystemLibrary.K2_SetTimerDelegate` (delegate `Spawn Enemy`) (`self.SpawnCooldown`))
  (`self.UpdateSpawnCooldownAndSpawners`)
  (`self.Spawn Enemy`))

(fn `GetRandomSpawnPoint`
  (returns (Location :type "Vector Structure"))
  (bind _outitem (`KismetArrayLibrary.Array_RandomFromStream` (`self.ActiveSpawners`) (`self.RandomStream`)))
  (bind _spawn_volume (`/Game/AstroChivalry/Blueprints/AI/Spawner/BP_EnemySpawner.Spawn Volume` _outitem))
  (`/Engine/EditorBlueprintResources/StandardMacros.IsValid` _outitem
    (:`Is Valid`
      (return (`KismetMathLibrary.RandomPointInBoundingBox` (`SceneComponent.K2_GetComponentLocation` _spawn_volume) (`BoxComponent.GetScaledBoxExtent` _spawn_volume))))))

(fn `Initialize`
  (bind _outactors (`GameplayStatics.GetAllActorsOfClass` "/Game/AstroChivalry/Blueprints/AI/Spawner/BP_EnemySpawner.BP_EnemySpawner_C"))
  (bind _output_get (set `self.SpawnersREF` _outactors))
  (while (> (`self.InitialActiveSpawners`) (`KismetArrayLibrary.Array_Length` (`self.ActiveSpawners`)))
    (`KismetArrayLibrary.Array_AddUnique` (`self.ActiveSpawners`) (`KismetArrayLibrary.Array_Random` _output_get)))
  (`KismetMathLibrary.SetRandomStreamSeed` (`self.RandomStream`) (`self.Seed`)))

(fn `UpdateSpawnCooldownAndSpawners`
  (locals (HasAdded :type Boolean))
  (bind _result (`/Engine/EditorBlueprintResources/StandardMacros.DecrementFloat` (`self.SpawnCooldown`))
    (:`  `
      (set `self.SpawnCooldown` _result)
      (for _array_element (`self.SpawnersREF`)
        (if (not (`local.HasAdded`))
          (`KismetArrayLibrary.Array_AddUnique` (`self.ActiveSpawners`) _array_element)
          (set `local.HasAdded` true))))))

(fn `UserConstructionScript`)
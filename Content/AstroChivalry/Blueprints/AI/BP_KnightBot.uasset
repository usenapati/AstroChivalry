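; BP_KnightBot is a knight AI bot that carries a musket and inherits its behavior from a parent bot class.
; The construction script registers its weapon component as the parent's musket weapon and flags it as musket-armed.
; On death it runs the parent logic, then detaches the weapon and switches it to physics-only simulation so it drops.
; Damage handling passes straight to the parent.
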(event `self.ReceiveAnyDamage`
  (params (Damage :type "Float (single-precision)") (DamageType :type "DamageType Object Reference") (InstigatedBy :type "Controller Object Reference") (DamageCauser :type "Actor Object Reference"))
  (`parent.ReceiveAnyDamage` Damage DamageType InstigatedBy DamageCauser))

(event `self.BotDeath`
  (bind _bp_weapon_component (`self.BP_Weapon_Component`))
  (`parent.BotDeath`)
  (`SceneComponent.K2_DetachFromComponent` _bp_weapon_component "KeepRelative" "KeepRelative" "KeepRelative" true)
  (`PrimitiveComponent.SetCollisionEnabled` _bp_weapon_component "PhysicsOnly")
  (`PrimitiveComponent.SetSimulatePhysics` _bp_weapon_component true))

(fn `UserConstructionScript`
  (`parent.UserConstructionScript`)
  (set `self.MusketWeapon` (`self.BP_Weapon_Component`))
  (set `self.HasMusket` true))
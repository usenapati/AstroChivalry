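; Health pickup actor that restores a fixed amount of health to the first-person player character on overlap.
; A looping timeline animates the Cube mesh's relative position and yaw as an idle effect.
; On pickup, it disables collision and hides the cube, then a timer re-enables both a few seconds later so the pickup respawns.
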(event `self.ReceiveBeginPlay`
  (bind (_direction _position _rotation__z_) (`Timeline|PickupEffectTimeline` :!label _label)
    (:`Update`
      (`SceneComponent.K2_SetRelativeLocationAndRotation` (`self.Cube`) _position (`KismetMathLibrary.MakeRotator` 0.0 0.0 _rotation__z_) false false))
    (:`Finished`
      (goto _label :!via `PlayFromStart`))))

(event `self.Collision.OnComponentBeginOverlap`
  (params (OverlappedComponent :type "PrimitiveComponent Object Reference") (OtherActor :type "Actor Object Reference") (OtherComp :type "PrimitiveComponent Object Reference") (OtherBodyIndex :type Integer) (bFromSweep :type Boolean) (SweepResult :type "HitResult Structure (by ref)"))
  (bind _asbp_first_person_character (cast `/Game/FirstPerson/Blueprints/BP_FirstPersonCharacter` OtherActor))
  (`/Game/FirstPerson/Blueprints/BP_FirstPersonCharacter.RestoreHealth` _asbp_first_person_character 50.0)
  (`PrimitiveComponent.SetCollisionEnabled` (`self.Collision`) "NoCollision")
  (`SceneComponent.SetVisibility` (`self.Cube`) false false)
  (`KismetSystemLibrary.K2_SetTimerDelegate` (delegate `PickupRespawn`) 5.0))

(event `PickupRespawn`
  (`PrimitiveComponent.SetCollisionEnabled` (`self.Collision`) "QueryOnly")
  (`SceneComponent.SetVisibility` (`self.Cube`) true false))

(fn `UserConstructionScript`)
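; Game mode for AstroChivalry that runs a timed round, won when the countdown ends.
; BeginPlay starts a three-minute timer that calls EndRound to flag the round as won.
; LoseRound, which is not called within this graph, cancels that timer and flags a loss.
; Both outcomes switch input to UI-only, show the cursor and freeze the game with zero global time dilation.
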(event `self.ReceiveBeginPlay`
  (bind _returnvalue (`KismetSystemLibrary.K2_SetTimer` null "EndRound" 180.0))
  (set `self.GameTimer` _returnvalue))

(fn `EndRound`
  (bind _returnvalue (`GameplayStatics.GetPlayerController` 0))
  (`WidgetBlueprintLibrary.SetInputMode_UIOnlyEx` _returnvalue null)
  (set `PlayerController.bShowMouseCursor` true _returnvalue)
  (set `self.WonRound` true)
  (`GameplayStatics.SetGlobalTimeDilation` 0.0))

(fn `LoseRound`
  (bind _returnvalue (`GameplayStatics.GetPlayerController` 0))
  (`KismetSystemLibrary.K2_ClearTimer` null "EndRound")
  (`WidgetBlueprintLibrary.SetInputMode_UIOnlyEx` _returnvalue null)
  (set `PlayerController.bShowMouseCursor` true _returnvalue)
  (set `self.LostRound` true)
  (`GameplayStatics.SetGlobalTimeDilation` 0.0))

(fn `UserConstructionScript`)
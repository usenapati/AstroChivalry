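; KoboldObjective is the objective actor whose destruction makes KoboldGameMode lose the round.
; Its EnemyDetectSphere, on activation, calls FoundObjective on every Bot_AIController in the world.
; Once the force field is destroyed, a BP_Bot entering the sphere has its controller told it found this objective.
; A bot leaving then triggers LostStructure on its controller.
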(event `self.ReceiveTick`
  (params (DeltaSeconds :type "Float (single-precision)"))
  (`parent.ReceiveTick` DeltaSeconds))

(event `self.ReceiveDestroyed`
  (bind _askobold_game_mode (cast `/Game/AstroChivalry/Blueprints/KoboldGameMode` (`GameplayStatics.GetGameMode`)))
  (`/Game/AstroChivalry/Blueprints/KoboldGameMode.LoseRound` _askobold_game_mode))

(event `self.EnemyDetectSphere.OnComponentActivated`
  (params (Component :type "ActorComponent Object Reference") (bReset :type Boolean))
  (bind _outactors (`GameplayStatics.GetAllActorsOfClass` "/Game/AstroChivalry/Blueprints/AI/Bot_AIController.Bot_AIController_C"))
  (for _array_element _outactors
    (`/Game/AstroChivalry/Blueprints/AI/Bot_AIController.FoundObjective` _array_element null)))

(event `self.EnemyDetectSphere.OnComponentBeginOverlap`
  (params (OverlappedComponent :type "PrimitiveComponent Object Reference") (OtherActor :type "Actor Object Reference") (OtherComp :type "PrimitiveComponent Object Reference") (OtherBodyIndex :type Integer) (bFromSweep :type Boolean) (SweepResult :type "HitResult Structure (by ref)"))
  (if (`self.IsForceFieldDestroyed`)
    (bind _asbp_bot (cast `/Game/AstroChivalry/Blueprints/AI/BP_Bot` OtherActor))
    (if true
      (`KismetSystemLibrary.PrintString` "Entered Sphere")
      (bind _asbot_aicontroller (cast `/Game/AstroChivalry/Blueprints/AI/Bot_AIController` (`AIBlueprintHelperLibrary.GetAIController` _asbp_bot)))
      (`/Game/AstroChivalry/Blueprints/AI/Bot_AIController.FoundObjective` _asbot_aicontroller self))))

(event `self.EnemyDetectSphere.OnComponentEndOverlap`
  (params (OverlappedComponent :type "PrimitiveComponent Object Reference") (OtherActor :type "Actor Object Reference") (OtherComp :type "PrimitiveComponent Object Reference") (OtherBodyIndex :type Integer))
  (if (`self.IsForceFieldDestroyed`)
    (bind _asbp_bot (cast `/Game/AstroChivalry/Blueprints/AI/BP_Bot` OtherActor))
    (`KismetSystemLibrary.PrintString` "Left Sphere")
    (bind _asbot_aicontroller (cast `/Game/AstroChivalry/Blueprints/AI/Bot_AIController` (`AIBlueprintHelperLibrary.GetAIController` _asbp_bot)))
    (`/Game/AstroChivalry/Blueprints/AI/Bot_AIController.LostStructure` _asbot_aicontroller)))

(fn `UserConstructionScript`
  (`parent.UserConstructionScript`))
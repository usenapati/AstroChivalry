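; Generator is a structure actor that enemy bots can detect, linked to the level's Forcefield.
; On BeginPlay it finds and caches the Forcefield, then applies fixed damage to it when the generator is destroyed.
; Bots entering or leaving its EnemyDetectSphere have their Bot_AIController notified via FoundStructure or LostStructure, with debug prints on each.
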(event `self.ReceiveBeginPlay`
  (`parent.ReceiveBeginPlay`)
  (bind _returnvalue (`GameplayStatics.GetActorOfClass` "/Game/AstroChivalry/Blueprints/Forcefield.Forcefield_C"))
  (set `self.ForceField` _returnvalue))

(event `self.ReceiveDestroyed`
  (bind _forcefield (`self.ForceField`))
  (`/Engine/EditorBlueprintResources/StandardMacros.IsValid` _forcefield
    (:`Is Valid`
      (`GameplayStatics.ApplyDamage` _forcefield 30.0 null self))))

(event `self.EnemyDetectSphere.OnComponentBeginOverlap`
  (params (OverlappedComponent :type "PrimitiveComponent Object Reference") (OtherActor :type "Actor Object Reference") (OtherComp :type "PrimitiveComponent Object Reference") (OtherBodyIndex :type Integer) (bFromSweep :type Boolean) (SweepResult :type "HitResult Structure (by ref)"))
  (bind _asbp_bot (cast `/Game/AstroChivalry/Blueprints/AI/BP_Bot` OtherActor))
  (`KismetSystemLibrary.PrintString` "Entered Sphere")
  (bind _asbot_aicontroller (cast `/Game/AstroChivalry/Blueprints/AI/Bot_AIController` (`AIBlueprintHelperLibrary.GetAIController` _asbp_bot)))
  (`/Game/AstroChivalry/Blueprints/AI/Bot_AIController.FoundStructure` _asbot_aicontroller self))

(event `self.EnemyDetectSphere.OnComponentEndOverlap`
  (params (OverlappedComponent :type "PrimitiveComponent Object Reference") (OtherActor :type "Actor Object Reference") (OtherComp :type "PrimitiveComponent Object Reference") (OtherBodyIndex :type Integer))
  (bind _asbp_bot (cast `/Game/AstroChivalry/Blueprints/AI/BP_Bot` OtherActor))
  (if true
    (`KismetSystemLibrary.PrintString` "Left Sphere")
    (bind _asbot_aicontroller (cast `/Game/AstroChivalry/Blueprints/AI/Bot_AIController` (`AIBlueprintHelperLibrary.GetAIController` _asbp_bot)))
    (`/Game/AstroChivalry/Blueprints/AI/Bot_AIController.LostStructure` _asbot_aicontroller)))

(fn `UserConstructionScript`
  (`parent.UserConstructionScript`))
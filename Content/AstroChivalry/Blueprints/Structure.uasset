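; Destructible structure actor that loses health from any damage not caused by the player pawn.
; At zero health it hides the mesh, disables collision and plays a destruction particle system, then destroys itself when the effect finishes.
; A detection sphere notifies bot AI controllers when the structure is found or lost.
; The construction script passes a dynamic instance of the mesh material to the destruction effect.
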(event `self.ReceiveBeginPlay`)

(event `self.ReceiveAnyDamage`
  (params (Damage :type "Float (single-precision)") (DamageType :type "DamageType Object Reference") (InstigatedBy :type "Controller Object Reference") (DamageCauser :type "Actor Object Reference"))
  (bind _mesh (`self.Mesh`))
  (if (!= DamageCauser (`GameplayStatics.GetPlayerPawn` 0))
    (bind _output_get (set `self.Health` (- (`self.Health`) Damage)))
    (if (<= _output_get 0.0)
      (`SceneComponent.SetVisibility` _mesh false false)
      (`PrimitiveComponent.SetCollisionEnabled` _mesh "NoCollision")
      (`ActorComponent.Activate` (`self.ObjectDestruction`) true))))

(event `self.ObjectDestruction.OnSystemFinished`
  (params (PSystem :type "NiagaraComponent Object Reference"))
  (`self.K2_DestroyActor`))

(event `self.EnemyDetectSphere.OnComponentBeginOverlap`
  (params (OverlappedComponent :type "PrimitiveComponent Object Reference") (OtherActor :type "Actor Object Reference") (OtherComp :type "PrimitiveComponent Object Reference") (OtherBodyIndex :type Integer) (bFromSweep :type Boolean) (SweepResult :type "HitResult Structure (by ref)"))
  (if (== OtherActor "/Game/AstroChivalry/Blueprints/AI/BP_Bot.BP_Bot")
    (`KismetSystemLibrary.PrintString` "Entered Sphere")
    (bind _asbot_aicontroller (cast `/Game/AstroChivalry/Blueprints/AI/Bot_AIController` (`AIBlueprintHelperLibrary.GetAIController` OtherActor)))
    (`/Game/AstroChivalry/Blueprints/AI/Bot_AIController.FoundStructure` _asbot_aicontroller self)))

(event `self.EnemyDetectSphere.OnComponentEndOverlap`
  (params (OverlappedComponent :type "PrimitiveComponent Object Reference") (OtherActor :type "Actor Object Reference") (OtherComp :type "PrimitiveComponent Object Reference") (OtherBodyIndex :type Integer))
  (if (== null OtherActor)
    (`KismetSystemLibrary.PrintString` "Left Sphere")
    (bind _asbot_aicontroller (cast `/Game/AstroChivalry/Blueprints/AI/Bot_AIController` (`AIBlueprintHelperLibrary.GetAIController` OtherActor)))
    (`/Game/AstroChivalry/Blueprints/AI/Bot_AIController.LostStructure` _asbot_aicontroller)))

(fn `UserConstructionScript`
  (bind _mesh (`self.Mesh`))
  (bind _returnvalue (`PrimitiveComponent.CreateDynamicMaterialInstance` _mesh 0 (`PrimitiveComponent.GetMaterial` _mesh 0) "None"))
  (`NiagaraComponent.SetVariableMaterial` (`self.ObjectDestruction`) "test" _returnvalue)
  (`KismetSystemLibrary.PrintString` "Hello"))
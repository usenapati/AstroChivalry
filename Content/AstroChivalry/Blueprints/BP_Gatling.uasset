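; BP_Gatling is an auto-firing gatling turret that targets actors tagged "Enemy" within its TargetRadius.
; Tick yaws the mesh toward the first target and launches GatlingProjectiles from a socket, throttled by a DoOnce and reset timer, with velocity scaled by target distance.
; Damage passing a player-pawn check drains Health; at zero the mesh hides and ObjectDestruction plays, using its dynamic material, before the actor is destroyed.
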(event `self.ReceiveTick`
  (params (DeltaSeconds :type "Float (single-precision)"))
  (bind _staticmesh (`self.StaticMesh`))
  (bind (_returnvalue_roll _returnvalue_pitch) (`KismetMathLibrary.BreakRotator` (`SceneComponent.K2_GetComponentRotation` _staticmesh)))
  (bind (_returnvalue_roll_2 _returnvalue_pitch_2 _returnvalue_yaw) (`KismetMathLibrary.BreakRotator` (`KismetMathLibrary.FindLookAtRotation` (`self.K2_GetActorLocation`) (`self.K2_GetActorLocation` (`|GetArrayItem` (`self.Targets`))))))
  (if (`KismetArrayLibrary.Array_IsNotEmpty` (`self.Targets`))
    (`SceneComponent.K2_SetWorldRotation` _staticmesh (`KismetMathLibrary.MakeRotator` _returnvalue_roll _returnvalue_pitch (- _returnvalue_yaw 270.0)) false false)
    (`/Engine/EditorBlueprintResources/StandardMacros.DoOnce` false :!label _label
      (:`Completed`
        (bind _returnvalue (`|SpawnActorFromClass` "/Game/AstroChivalry/Blueprints/GatlingProjectile.GatlingProjectile_C" (`KismetMathLibrary.MakeTransform` (`SceneComponent.GetSocketLocation` (`self.StaticMesh`) "ProjectileSpawn") (`KismetMathLibrary.MakeRotator` _returnvalue_roll_2 _returnvalue_pitch_2 _returnvalue_yaw)) "Undefined" "MultiplyWithRoot" null null))
        (`PrimitiveComponent.SetPhysicsLinearVelocity` (`/Game/AstroChivalry/Blueprints/GatlingProjectile.Bullet` _returnvalue) (* (- (`self.K2_GetActorLocation` (`|GetArrayItem` (`self.Targets`))) (`SceneComponent.GetSocketLocation` (`self.StaticMesh`) "ProjectileSpawn")) 2.0) false "None")
        (`KismetSystemLibrary.K2_SetTimerDelegate` (delegate `ResetCannon`) 0.1)))))

(event `self.TargetRadius.OnComponentBeginOverlap`
  (params (OverlappedComponent :type "PrimitiveComponent Object Reference") (OtherActor :type "Actor Object Reference") (OtherComp :type "PrimitiveComponent Object Reference") (OtherBodyIndex :type Integer) (bFromSweep :type Boolean) (SweepResult :type "HitResult Structure (by ref)"))
  (if (`KismetArrayLibrary.Array_Contains` (`Actor.Tags` OtherActor) "Enemy")
    (`KismetArrayLibrary.Array_Add` (`self.Targets`) OtherActor)))

(event `ResetCannon`
  (goto _label :!via `Reset`))

(event `self.TargetRadius.OnComponentEndOverlap`
  (params (OverlappedComponent :type "PrimitiveComponent Object Reference") (OtherActor :type "Actor Object Reference") (OtherComp :type "PrimitiveComponent Object Reference") (OtherBodyIndex :type Integer))
  (if (`KismetArrayLibrary.Array_Contains` (`self.Targets`) OtherActor)
    (`KismetArrayLibrary.Array_RemoveItem` (`self.Targets`) OtherActor)))

(event `self.ReceiveAnyDamage`
  (params (Damage :type "Float (single-precision)") (DamageType :type "DamageType Object Reference") (InstigatedBy :type "Controller Object Reference") (DamageCauser :type "Actor Object Reference"))
  (bind _staticmesh (`self.StaticMesh`))
  (if (!= null (`GameplayStatics.GetPlayerPawn` 0))
    (bind _output_get (set `self.Health` (- (`self.Health`) Damage)))
    (if (<= _output_get 0.0)
      (`SceneComponent.SetVisibility` _staticmesh false true)
      (`PrimitiveComponent.SetCollisionEnabled` _staticmesh "NoCollision")
      (`ActorComponent.Activate` (`self.ObjectDestruction`) true))))

(event `self.ObjectDestruction.OnSystemFinished`
  (params (PSystem :type "NiagaraComponent Object Reference"))
  (`self.K2_DestroyActor`))

(fn `UserConstructionScript`
  (bind _returnvalue (`PrimitiveComponent.CreateDynamicMaterialInstance` (`self.StaticMesh`) 0 null "None"))
  (`NiagaraComponent.SetVariableMaterial` (`self.ObjectDestruction`) "test" _returnvalue)
  (`KismetSystemLibrary.PrintString` "Hello"))
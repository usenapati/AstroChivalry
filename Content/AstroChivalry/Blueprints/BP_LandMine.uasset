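; Land mine actor that explodes when anything other than the first player's pawn enters its box trigger.
; On trigger it plays an explosion effect and sound, then destroys its box and mesh components before querying overlapping actors.
; It applies fixed damage to each returned actor except that pawn, crediting the player as damage causer, then destroys itself.
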(event `self.Box.OnComponentBeginOverlap`
  (params (OverlappedComponent :type "PrimitiveComponent Object Reference") (OtherActor :type "Actor Object Reference") (OtherComp :type "PrimitiveComponent Object Reference") (OtherBodyIndex :type Integer) (bFromSweep :type Boolean) (SweepResult :type "HitResult Structure (by ref)"))
  (bind _returnvalue (`self.K2_GetActorLocation`))
  (bind _returnvalue_2 (`GameplayStatics.GetPlayerPawn` 0))
  (if (not (== OtherActor (`GameplayStatics.GetPlayerPawn` 0)))
    (`GameplayStatics.SpawnEmitterAtLocation` "/Game/StarterContent/Particles/P_Explosion.P_Explosion" _returnvalue)
    (`GameplayStatics.PlaySoundAtLocation` "/Game/StarterContent/Audio/Explosion01.Explosion01" _returnvalue (struct) 1.0 1.0 0.0 null null null null)
    (`ActorComponent.K2_DestroyComponent` (`self.Box`))
    (`ActorComponent.K2_DestroyComponent` (`self.StaticMesh`))
    (for _array_element (`self.GetOverlappingActors` null)
      (if (not (== _array_element _returnvalue_2))
        (`GameplayStatics.ApplyDamage` _array_element 150.0 null _returnvalue_2)))
    (`self.K2_DestroyActor`)))

(fn `UserConstructionScript`)